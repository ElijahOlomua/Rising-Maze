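; Character component that adds Titanfall-style wall running, with wall jumps and camera roll.
; A looping timer started in Start line-traces right, then left, for near-vertical walls while falling, launching the character along the surface and easing gravity toward a target.
; Ending a run restores gravity and briefly suppresses re-entry, while jumping launches off the wall normal.
; Tick interpolates control rotation roll according to the wall side.
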(event `Land`
  (`self.WallRunEnd` 0.0)
  (set `self.Wall run suppressed` false))

(event `Set wall run suppression`
  (`KismetSystemLibrary.K2_ClearTimer` null "Set wall run suppression")
  (set `self.Wall run suppressed` false))

(event `Jump`
  (`self.WallRunJump`))

(event `Start`
  (params (Character :type "Character Object Reference"))
  (bind _output_get (set `self.CharacterRef` Character))
  (bind _output_get_2 (set `self.CharacterMovementRef` (`Character.CharacterMovement` _output_get)))
  (set `self.DefaultGravityRef` (`CharacterMovementComponent.GravityScale` _output_get_2))
  (`KismetSystemLibrary.K2_SetTimerDelegate` (delegate `Update`) 0.02 true))

(event `Update`
  (if (not (`self.Wall run suppressed`))
    (`self.WallRunUpdate`)))

(event `self.ReceiveTick`
  (params (DeltaSeconds :type "Float (single-precision)"))
  (`self.Camera tick`))

(fn `Camera tick`
  (if (`self.WallRunningLeft`)
    (`self.Camera tilt` 15.0)
    (elif (`self.WallRunningRight`)
      (`self.Camera tilt` -15.0)
      (else
        (`self.Camera tilt` 0.0)))))

(fn `Camera tilt`
  (params (`Target X (roll)` :type "Float (double-precision)"))
  (bind _returnvalue (`Controller.GetControlRotation` (`Pawn.GetController` (`self.CharacterRef`))))
  (`Controller.SetControlRotation` (`Pawn.GetController` (`self.CharacterRef`)) (`KismetMathLibrary.RInterpTo` _returnvalue (`KismetMathLibrary.MakeRotator` `Target X (roll)` (.pitch _returnvalue) (.yaw _returnvalue)) (`GameplayStatics.GetWorldDeltaSeconds`) 10.0)))

(fn `Suppress wall run`
  (params (Delay :type "Float (double-precision)"))
  (set `self.Wall run suppressed` true)
  (`KismetSystemLibrary.K2_SetTimer` null "Set wall run suppression" Delay))

(fn `WallRunEnd`
  (params (`Reset time` :type "Float (double-precision)"))
  (if (`self.WallRunning`)
    (set `self.WallRunning` false)
    (set `self.WallRunningLeft` false)
    (set `self.WallRunningRight` false)
    (set `CharacterMovementComponent.GravityScale` (`self.DefaultGravityRef`) (`self.CharacterMovementRef`))
    (`self.Suppress wall run` (`local.Reset time`))))

(fn `WallRunJump`
  (bind (_wall_run_normal_x _wall_run_normal_y) (`KismetMathLibrary.BreakVector` (`self.Wall run normal`)))
  (bind _wall_run_jump_off_force (`self.Wall run jump off force`))
  (if (`self.WallRunning`)
    (`self.WallRunEnd` 0.35)
    (`Character.LaunchCharacter` (`self.CharacterRef`) (`KismetMathLibrary.MakeVector` (* _wall_run_jump_off_force _wall_run_normal_x) (* _wall_run_jump_off_force _wall_run_normal_y) (`self.Wall run jump height`)) false true)))

(fn `WallRunMovement`
  (params (Start :type "Vector Structure") (End :type "Vector Structure") (WallRunDirection :type "Float (double-precision)"))
  (returns (`On wall` :type Boolean))
  (bind _outhit (`KismetSystemLibrary.LineTraceSingle` :`Start` Start :`End` End :`TraceChannel` "TraceTypeQuery1" :`DrawDebugType` "ForOneFrame"))
  (if (`GameplayStatics.BreakHitResult` _outhit)
    (bind (_returnvalue _out_hit_normal_vec) (`self.ValidWallRunVector` (`.Normal` (`GameplayStatics.BreakHitResult` _outhit))))
    (if (and (`NavMovementComponent.IsFalling` (`self.CharacterMovementRef`)) _returnvalue)
      (set `self.Wall run normal` _out_hit_normal_vec)
      (`Character.LaunchCharacter` (`self.CharacterRef`) (`self.Player to wall vector `) false false)
      (`Character.LaunchCharacter` (`self.CharacterRef`) (* (`KismetMathLibrary.Cross_VectorVector` (`self.Wall run normal`) (0.0 0.0 1.0)) (* (`self.Wall run speed`) (`local.WallRunDirection`))) true (not (`self.Wall run gravity`)))
      (return true)
      (else
        (return false)))
    (else
      (return false))))

(fn `WallRunUpdate`
  (bind _on_wall (`self.WallRunMovement` (`Actor.K2_GetActorLocation` (`self.CharacterRef`)) (`self.EndVectors`) -1.0))
  (if _on_wall
    (set `self.WallRunning` false)
    (set `self.WallRunningRight` true)
    (set `self.WallRunningLeft` false)
    (set `CharacterMovementComponent.GravityScale` (`KismetMathLibrary.FInterpTo` (`CharacterMovementComponent.GravityScale` (`self.CharacterMovementRef`)) (`self.Wall run target gravity`) (`GameplayStatics.GetWorldDeltaSeconds`) 10.0) (`self.CharacterMovementRef`) :!label _label)
    (elif (`self.WallRunningRight`)
      (`self.WallRunEnd` 1.0)
      (else
        (bind _on_wall_2 (`self.WallRunMovement` (`Actor.K2_GetActorLocation` (`self.CharacterRef`)) (`.LeftVector` (`self.EndVectors`)) 1.0))
        (if _on_wall_2
          (set `self.WallRunning` false)
          (set `self.WallRunningRight` false)
          (set `self.WallRunningLeft` true)
          (goto _label)
          (else
            (`self.WallRunEnd` 0.5)))))))